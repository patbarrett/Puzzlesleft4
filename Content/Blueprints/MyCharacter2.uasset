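; MyCharacter2 is a character with a toggleable spotlight flashlight and a destroy-then-spectate key.
; The Flashlight input switches on authority, reaching the intensity toggle directly or through a relay custom event on remotes, and construction starts the light dark.
; Releasing Z destroys the pawn owner and moves player zero's view to the first MyCharacter2 not equal to the controller, a self-check comparing character to controller.
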(event `Key|Z`
  (:`Released`
    (`self.K2_DestroyActor` (`PawnMovementComponent.GetPawnOwner`))
    (bind _outactors (`GameplayStatics.GetAllActorsOfClass` "MyCharacter2_C"))
    (for _array_element _outactors
      (`KismetSystemLibrary.PrintString` "Checking")
      (if (== _array_element (`self.GetController`))
        (`KismetSystemLibrary.PrintString` "Found Self")
        (else
          (`KismetSystemLibrary.PrintString` "Found Other")
          (`PlayerController.SetViewTargetWithBlend` (`GameplayStatics.GetPlayerController` 0) _array_element 0.0 "VTBlend_Linear" 0.0 false)
          (break))))))

(event `self.ReceiveBeginPlay`)

(event `CustomEvent_0`
  (if (`self.IsOn`)
    (`LightComponent.SetIntensity` (`self.SpotLight`) 0.0)
    (set `self.IsOn` false)
    (else
      (`LightComponent.SetIntensity` (`self.SpotLight`) 10000.0)
      (set `self.IsOn` true))))

(event `CustomEvent_1`
  (`self.CustomEvent_0` :!label _label))

(event `InputAction|Flashlight`
  (:`Pressed`
    (`/Engine/EditorBlueprintResources/ActorMacros.Switch Has Authority`
      (:`Authority`
        (goto _label))
      (:`Remote`
        (`self.CustomEvent_1`)))))

(fn `UserConstructionScript`
  (`LightComponent.SetIntensity` (`self.SpotLight`) 0.0))